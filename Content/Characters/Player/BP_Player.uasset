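; Player Blueprint that handles incoming damage with a brief invincibility window after each hit.
; AnyDamage and a custom damage event share one path, which passes damage to Stat.DecreaseHealth only when the player is not invincible.
; A hit sets the invincible flag and disables capsule collision, then a one-shot timer restores both after the duration set at BeginPlay.
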(event `self.TakeDamageBPEvenet`
  (params (Damage :type "Float (single-precision)") (DamageEvent :type "DamageEvent Structure (by ref)") (EventInstigator :type "Controller Object Reference") (DamageCauser :type "Actor Object Reference"))
  ;[1 1 1] AnyDamage(TakeDamage)
  (if (not (`self.IsInvincible`)) :!label _label
    (`StatComponent.DecreaseHealth` (`self.Stat`) Damage)
    (set `self.IsInvincible` true)
    (`PrimitiveComponent.SetCollisionEnabled` (`self.CapsuleComponent`) "NoCollision")
    (`KismetSystemLibrary.K2_SetTimerDelegate` (delegate `SetInvinsibleOff`) (`self.InvincibleTime`))))

(event `self.ReceiveAnyDamage`
  (params (Damage :type "Float (single-precision)") (DamageType :type "DamageType Object Reference") (InstigatedBy :type "Controller Object Reference") (DamageCauser :type "Actor Object Reference"))
  ;[1 1 1] AnyDamage(TakeDamage)
  (goto _label))

(event `SetInvinsibleOff`
  ;[1 1 1] AnyDamage(TakeDamage)
  (set `self.IsInvincible` false)
  (`PrimitiveComponent.SetCollisionEnabled` (`self.CapsuleComponent`) "QueryAndPhysics"))

(event `self.ReceiveBeginPlay`
  (set `self.InvincibleTime` 1.0)
  (set `self.IsInvincible` false))

(fn `UserConstructionScript`)